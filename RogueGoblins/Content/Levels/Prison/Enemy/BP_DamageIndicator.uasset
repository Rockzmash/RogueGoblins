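; BP_DamageIndicator is a floating damage number actor, shown through a widget component that receives the Damage value on BeginPlay.
; It picks a randomized end point above and to the side, using up and right vectors obtained from the player character through an interface.
; A Timeline lerps the actor to that point, then destroys it when finished.
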(event EventBeginPlay
  (Class|BPIDamageIndicator|IFSetDamage(Message) (UserInterface|GetWidget (Variables|Default|GetDamage%20Widget)) (Variables|Default|GetDamage))
  (bind _output_get (Variables|Default|SetStartPos (Transformation|GetActorLocation)))
  (bind (_up_vector _right_vector) (Class|BPIPlayer|IFGetVectors(Message) (Game|GetPlayerCharacter 0)))
  (Variables|Default|SetEndPos (+ _output_get (* _up_vector (Math|Random|RandomFloatinRange 4e+01 5e+01)) (* _right_vector (Math|Random|RandomFloatinRange 2e+01 3e+01))))
  (bind _newtrack_0 (Timeline|Timeline Play)
    (:Update
      (Transformation|SetActorLocation (Math|Vector|Lerp(Vector) (Variables|Default|GetStartPos) (Variables|Default|GetEndPos) _newtrack_0) false false))
    (:Finished
      (Actor|DestroyActor))))

(fn ConstructionScript)