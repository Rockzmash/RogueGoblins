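; BP_Goblin_Brute is a goblin player Blueprint with melee attack events, extending parent logic.
; BeginPlay disables weapon collision.
; PrimaryAttack plays a sword-swing montage, waits, then sphere-overlaps at a scaled forward vector without actor location, drawing debug, and damages "Enemy"-tagged actors with a random crit multiplier.
; SecondaryAttack is a stub with an unassigned montage and delay; both attacks gate on BlsAttacking being true.
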(event EventBeginPlay
  (|CallParentFunction)
  (Collision|SetCollisionEnabled (Variables|Default|GetWeapon%20Collision) "NoCollision"))

(event EventPrimaryAttack
  (bind _returnvalue (Transformation|GetActorForwardVector))
  (bind _damage (Variables|Default|GetDamage))
  (bind _ability_size (Variables|Default|GetAbility%20Size))
  (bind _returnvalue_2 (* _returnvalue 3e+01))
  (if (Variables|Default|GetblsAttacking)
    (Variables|Default|SetblsAttacking true)
    (bind _returnvalue_3 (Animation|PlayAnimMontage "/Game/Characters/Mannequins/Anims/Unarmed/Attack/AM_Sword_Swing.AM_Sword_Swing" 1.0 "None"))
    (Utilities|FlowControl|Delay _returnvalue_3)
    (Rendering|Debug|DrawDebugSphere _returnvalue_2 _ability_size 12 "(R=1.000000,G=1.000000,B=1.000000,A=1.000000)" 1e+01)
    (bind _outactors (Collision|SphereOverlapActors _returnvalue_2 _ability_size (Utilities|Array|MakeArray "ObjectTypeQuery3" "ObjectTypeQuery2") 0))
    (for _array_element _outactors
      (if (Actor|ActorHasTag _array_element "Enemy")
        (if (<= (Math|Random|RandomFloatinRange 0.0 1e+02) (Variables|Default|GetCrit%20Chance))
          (Game|Damage|ApplyDamage _array_element (* _damage (Variables|Default|GetCrit%20DMG%20Mult)) 0 0) ; Crit Damage
          (else
            (Game|Damage|ApplyDamage _array_element _damage 0 0) ; Regular Damage
          ))
        (Utilities|Time|SetTimerbyEvent 0 0.5)
        (Variables|Default|SetblsAttacking false)))))

(event EventSecondaryAttack
  (if (Variables|Default|GetblsAttacking)
    (Variables|Default|SetblsAttacking true)
    (bind _returnvalue (Animation|PlayAnimMontage 0 1.0 "None"))
    (Utilities|FlowControl|Delay _returnvalue)))

(fn ConstructionScript
  (|CallParentFunction))